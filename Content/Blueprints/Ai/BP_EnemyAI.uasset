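; Enemy AI controller that hunts sighted actors tagged "Player" and otherwise wanders between BP_TaskNode points.
; A looping timer checks sight perception, setting Target, focus and Hunt state, then starting a move to the target when newly acquired.
; Losing a target requests Search, which SetState turns into Idle, where the Wander Around task moves to random points.
; Tick prints the current state and task for debugging.
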(event `self.ReceiveBeginPlay`
  (`KismetSystemLibrary.K2_SetTimerDelegate` (delegate `UpdateAi`) 0.1 true)
  (bind _outactors (`GameplayStatics.GetAllActorsOfClass` "/Game/Blueprints/Ai/Tasks/BP_TaskNode.BP_TaskNode_C"))
  (set `self.WalkingPoints` _outactors))

(event `UpdateAi`
  (bind _outitem (`KismetArrayLibrary.Array_Random` (`self.WalkingPoints`)))
  (bind _outactors (`AIPerceptionComponent.GetPerceivedActors` (`self.AIPerception`) "/Script/AIModule.AISense_Sight"))
  (`|ExecutionSequence`
    (:`then_0`
      (if (== (`KismetArrayLibrary.Array_Find` _outactors (`self.Target`)) -1)
        (set `self.Found` false)
        (for _array_element _outactors
          (if (!= (`KismetArrayLibrary.Array_Find` (`Actor.Tags` _array_element) "Player") -1)
            (bind _output_get (set `self.Target` _array_element))
            (set `self.Found` true)
            (`self.K2_SetFocus` _output_get)
            (`self.SetState` "NewEnumerator2")))
        (if (not (`self.Found`))
          (`self.SetState` "NewEnumerator1")
          (set `self.Target` null)
          (`self.K2_SetFocus` null)
          (else
            (`AITask_MoveTo.AIMoveTo` self (0.0 0.0 0.0) (`self.Target`) -1.0 "Default" "Default" true true true)))))
    (:`then_1`
      (switch `/Game/Blueprints/Ai/States/E_State` (`self.CurrentState`)
        (:`NewEnumerator0`
          (switch `/Game/Blueprints/Ai/States/Idle/E_IdleAction` (`self.CurrentTask`)
            (:`NewEnumerator4`
              (if (not (`KismetSystemLibrary.IsValid` (`self.CurrentWanderTarget`)))
                (set `self.CurrentWanderTarget` _outitem)
                (`AITask_MoveTo.AIMoveTo` self (0.0 0.0 0.0) _outitem
                  (:`OnMoveFinished`
                    (set `self.CurrentWanderTarget` null)))))))))))

(event `self.ReceiveTick`
  (params (DeltaSeconds :type "Float (single-precision)"))
  (`KismetSystemLibrary.PrintString` (`KismetStringLibrary.Concat_StrStr` (`|GetEnumeratorNameAsString` (`self.CurrentState`)) "->" (`|GetEnumeratorNameAsString` (`self.CurrentTask`))) true false (struct :`G` 0.66 :`B` 1.0 :`A` 1.0) DeltaSeconds))

(fn `SetState`
  (params (DesiredState :type "/Game/Blueprints/Ai/States/E_State Enum" :default "NewEnumerator0"))
  (if (`|EnumEquality` DesiredState "NewEnumerator1")
    (`/Engine/EditorBlueprintResources/StandardMacros.IsValid` (`self.Target`)
      (:`Is Valid`
        (set `self.CurrentState` "NewEnumerator0")))
    (else
      (set `self.CurrentState` DesiredState))))

(fn `UserConstructionScript`)