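; BP_DoorBase is an interactable swinging door that toggles open and closed on Interact unless any entry in its Locks array is locked.
; A locked door plays a locked sound, while Open and Close play a move sound and run the Movement timeline forward or in reverse.
; The timeline drives the mesh's yaw up to 90 degrees and plays an end sound, with its play rate set from SpeedMultiplier at construction.
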(event `/Game/Blueprints/I_Interaction.Interact`
  (bind _isopen (`self.IsOpen`))
  (if (not (`self.IsLocked`))
    (if _isopen
      (`self.Close`)
      (else
        (`self.Open`)))
    (set `self.IsOpen` (not _isopen))
    (else
      (`GameplayStatics.PlaySoundAtLocation` (`self.LockedSound`) (`self.K2_GetActorLocation`) (struct) 1.0 1.0 0.0 "/Game/Sound/SC_Ambient.SC_Ambient" null null))))

(fn `Close`
  (`GameplayStatics.PlaySoundAtLocation` (`self.MoveSound`) (`self.K2_GetActorLocation`) (struct) 1.0 1.0 0.0 "/Game/Sound/SC_Ambient.SC_Ambient" null null)
  (`TimelineComponent.Reverse` (`self.Movement`)))

(fn `IsLocked`
  (returns (Is :type Boolean))
  (locals (Locked :type Boolean))
  (for _array_element (`self.Locks`)
    (if (`/Game/Blueprints/Item/BP_Lock.Locked` _array_element)
      (return true)))
  (return false))

(fn `Open`
  (`GameplayStatics.PlaySoundAtLocation` (`self.MoveSound`) (`self.K2_GetActorLocation`) (struct) 1.0 1.0 0.0 "/Game/Sound/SC_Ambient.SC_Ambient" null null)
  (`TimelineComponent.Play` (`self.Movement`)))

(fn `UserConstructionScript`
  (`TimelineComponent.SetPlayRate` (`self.Movement`) (`self.SpeedMultiplier`)))