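; BP_ItemBase is a base Blueprint for physical items that can be picked up and dropped.
; BePickedUp turns off the item mesh's collision and physics simulation, and BeDropped turns both back on.
; On mesh hits, if hit sounds are enabled, it plays a sound at the impact point when speed times mass reaches a minimum threshold.
; The Interact event is an empty stub.
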(event `/Game/Blueprints/I_Interaction.Interact`)

(event `self.ItemMesh.OnComponentHit`
  (params (HitComponent :type "PrimitiveComponent Object Reference") (OtherActor :type "Actor Object Reference") (OtherComp :type "PrimitiveComponent Object Reference") (NormalImpulse :type "Vector Structure") (Hit :type "HitResult Structure (by ref)"))
  ;[1 1 1] Hit
  (if (`self.PlayHitSounds`)
    (if (>= (* (`KismetMathLibrary.VSize` (`self.GetVelocity`)) (`PrimitiveComponent.GetMass` (`self.ItemMesh`))) (`self.MinHitPowerToPlaySound`))
      (`GameplayStatics.PlaySoundAtLocation` (`self.HitSound`) (`.Location` (`GameplayStatics.BreakHitResult` Hit)) (struct) 1.0 1.0 0.0 null null null))))

(fn `BeDropped`
  (bind _itemmesh (`self.ItemMesh`))
  (`PrimitiveComponent.SetCollisionEnabled` _itemmesh "QueryAndPhysics")
  (`PrimitiveComponent.SetSimulatePhysics` _itemmesh true))

(fn `BePickedUp`
  (bind _itemmesh (`self.ItemMesh`))
  (`PrimitiveComponent.SetCollisionEnabled` _itemmesh "NoCollision")
  (`PrimitiveComponent.SetSimulatePhysics` _itemmesh false))

(fn `UserConstructionScript`)