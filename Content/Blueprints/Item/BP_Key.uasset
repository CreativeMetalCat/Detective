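; BP_Key is a colored key item that the player picks up and uses on BP_Lock actors.
; On pickup it stores the holding BP_Player.
; Using it while held line-traces from the first-person camera out to the player's interaction distance and passes the key's Code to any lock hit.
; The construction script tints the mesh with the key's Color through a dynamic material instance.
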(event `/Game/Blueprints/I_Interaction.UseItem`
  (bind _player (`self.Player`))
  (bind _firstpersoncameracomponent (`DetectiveUE4Character.FirstPersonCameraComponent` _player))
  (bind _returnvalue (`SceneComponent.K2_GetComponentLocation` _firstpersoncameracomponent))
  ;[1 1 1] Use
  (`/Engine/EditorBlueprintResources/StandardMacros.IsValid` (`self.Holder`)
    (:`Is Valid`
      (bind _outhit (`KismetSystemLibrary.LineTraceSingle` :`Start` _returnvalue :`End` (+ _returnvalue (* (`SceneComponent.GetForwardVector` _firstpersoncameracomponent) (`/Game/Blueprints/Player/BP_Player.InteractionDistance` _player))) :`TraceChannel` "TraceTypeQuery1" :`DrawDebugType` "ForDuration"))
      (bind _asbp_lock (cast `/Game/Blueprints/Item/BP_Lock` (`.HitActor` (`GameplayStatics.BreakHitResult` _outhit))))
      (`/Game/Blueprints/Item/BP_Lock.UseKeyCode` _asbp_lock (`self.Code`)))))

(fn `BePickedUp`
  (params (Holder :type "Actor Object Reference"))
  (`parent.BePickedUp` Holder)
  (bind _asbp_player (cast `/Game/Blueprints/Player/BP_Player` Holder))
  (set `self.Player` _asbp_player))

(fn `UserConstructionScript`
  (bind _itemmesh (`self.ItemMesh`))
  (`parent.UserConstructionScript`)
  (`/Engine/EditorBlueprintResources/StandardMacros.IsValid` (`self.KeyPaint`)
    (:`Is Valid`
      _)
    (:`Is Not Valid`
      (bind _returnvalue (`PrimitiveComponent.CreateDynamicMaterialInstance` _itemmesh 0 (`PrimitiveComponent.GetMaterial` _itemmesh 0) "None"))
      (set `self.KeyPaint` _returnvalue)))
  (`MaterialInstanceDynamic.SetVectorParameterValue` (`self.KeyPaint`) "Color" (`KismetMathLibrary.Conv_ColorToLinearColor` (`self.Color`))))