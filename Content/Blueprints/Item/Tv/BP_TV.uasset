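; Television item that can be switched on and off, changing its screen material and its sound.
; The construction script applies the initial On state by setting the material in mesh slot 1 and whether TVSound auto-activates.
; Toggle flips On at runtime, swapping that material and playing or stopping the sound.
; The event graph holds only disabled default nodes, so Toggle is not called within this Blueprint.
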(fn `Toggle`
  (bind _returnvalue (`self.GetItemMesh`))
  (bind _tv_sound (`self.TV_Sound`))
  (if (`self.On`)
    ;[1 1 1] Turn off
    (`PrimitiveComponent.SetMaterial` _returnvalue 1 (`self.TurnedOffMaterial`))
    (`AudioComponent.Stop` _tv_sound)
    (set `self.On` false)
    (else
      ;[1 1 1] Turn on
      (`PrimitiveComponent.SetMaterial` _returnvalue 1 (`self.TurnedOnMaterial`))
      (`AudioComponent.Play` _tv_sound 0.0)
      (set `self.On` true))))

(fn `UserConstructionScript`
  (bind _returnvalue (`self.GetItemMesh`))
  (bind _tv_sound (`self.TV_Sound`))
  (`parent.UserConstructionScript`)
  (if (not (`self.On`))
    ;[1 1 1] Turn off
    (`PrimitiveComponent.SetMaterial` _returnvalue 1 (`self.TurnedOffMaterial`))
    (`ActorComponent.SetAutoActivate` _tv_sound false)
    (else
      ;[1 1 1] Turn on
      (`PrimitiveComponent.SetMaterial` _returnvalue 1 (`self.TurnedOnMaterial`))
      (`ActorComponent.SetAutoActivate` _tv_sound true))))